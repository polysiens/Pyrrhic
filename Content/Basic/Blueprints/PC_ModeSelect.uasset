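; Player controller for the game mode selection screen.
; On BeginPlay it creates the W_ModeSelect widget, adds it to the viewport and keeps a reference to it.
; It then feeds the widget's tree items from the AvailableGameModes held by Basic_GameInstance, switches to UI-only input focused on the widget and shows the mouse cursor.
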(event Custom|SpawnModeSelectUI
  (CallFunction|SpawnUI)
  (Default|InitialTreeItemData (Variables|Default|GetModeSelectUI) (Variables|/Game/Basic/Basic_GameInstance.Basic_GameInstance_C|GetAvailableGameModes (.AsBasic%20Game%20Instance (Utilities|Casting|CastToBasic_GameInstance (Game|GetGameInstance)))))
  (Input|SetInputModeUIOnly self (Variables|Default|GetModeSelectUI) "DoNotLock" false)
  (Variables|Default|SetbShowMouseCursor true))

(event EventBeginPlay
  (CallFunction|SpawnModeSelectUI))

(fn ConstructionScript)

(fn SpawnUI
  (bind _returnvalue (UserInterface|CreateWidget "/Game/Basic/Widgets/w_ModeSelect.w_ModeSelect_C" self))
  (UserInterface|Viewport|AddtoViewport _returnvalue 0)
  (Variables|Default|SetModeSelectUI _returnvalue))